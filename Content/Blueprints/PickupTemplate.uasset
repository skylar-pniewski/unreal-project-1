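; PickupTemplate is a pickup item actor that the first-person character can collect into an inventory and later use.
; BeginPlay builds a prompt widget and binds pickup to the character; trigger overlap shows the prompt and enables pickup.
; Pickup adds ItemInfo to the HUD inventory and hides the actor until UseAction applies stat boosts and destroys it.
; End-overlap cleanup is disconnected, and EnergyValue is computed from HealthValue.
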(event `self.ReceiveBeginPlay`
  (bind _iteminfo (`self.ItemInfo`))
  (bind _pickuptextreference (`self.PickupTextReference`))
  (bind (_item _itemimage _pickuptext) (break `/Game/Blueprints/InventoryStruct` _iteminfo))
  ;[1 1 1] Event BeginPlay
  (bind _returnvalue (`|CreateWidget` "/Game/UMG/PickupText.PickupText_C"))
  (set `self.PickupTextReference` _returnvalue)
  (setmembers `/Game/Blueprints/InventoryStruct` :`StructRef` _iteminfo :`Item` self)
  (set `/Game/UMG/PickupText.PickupActor` _item _pickuptextreference)
  (set `/Game/UMG/PickupText.PickupText` _pickuptext _pickuptextreference)
  (bind _asfirst_person_character (cast `/Game/FirstPersonBP/Blueprints/FirstPersonCharacter` (`GameplayStatics.GetPlayerCharacter` 0)))
  (bind _output_get (set `self.CharacterReference` _asfirst_person_character))
  (add `/Game/FirstPersonBP/Blueprints/FirstPersonCharacter.PickupItem` _output_get (delegate `PickupItem_Event_0`)))

(event `self.Trigger.OnComponentBeginOverlap`
  (params (OverlappedComponent :type "PrimitiveComponent Object Reference") (OtherActor :type "Actor Object Reference") (OtherComp :type "PrimitiveComponent Object Reference") (OtherBodyIndex :type Integer) (bFromSweep :type Boolean) (SweepResult :type "HitResult Structure (by ref)"))
  ;[1 1 1] Overlap Trigger Script
  (cast `/Game/FirstPersonBP/Blueprints/FirstPersonCharacter` OtherActor)
  (`UserWidget.AddToViewport` (`self.PickupTextReference`) 0)
  (set `self.IsInRange?` true))

(event `PickupItem_Event_0`
  (bind _gamehudreference (`/Game/FirstPersonBP/Blueprints/FirstPersonCharacter.GameHUDReference` (`self.CharacterReference`)))
  ;[1 1 1] Pick up and add items to inventory and refresh it
  (if (and (`self.GetActorEnableCollision`) (`self.IsInRange?`))
    (`KismetArrayLibrary.Array_Add` (`/Game/UMG/GameHUD.Inventory` _gamehudreference) (`self.ItemInfo`))
    (`Widget.RemoveFromParent` (`self.PickupTextReference`))
    (`self.SetActorHiddenInGame` true)
    (`self.SetActorEnableCollision` false)
    (`/Game/UMG/GameHUD.RefreshInventory` _gamehudreference)))

(event `self.Trigger.OnComponentEndOverlap`
  (params (OverlappedComponent :type "PrimitiveComponent Object Reference") (OtherActor :type "Actor Object Reference") (OtherComp :type "PrimitiveComponent Object Reference") (OtherBodyIndex :type Integer))
  ;[1 1 1] Overlap Trigger Script
)

(event `/Game/Blueprints/ActionInterface.UseAction`
  (bind _characterreference (`self.CharacterReference`))
  (bind _healthvalue (`/Game/FirstPersonBP/Blueprints/FirstPersonCharacter.HealthValue` _characterreference))
  ;[1 1 1] Use Action
  (set `/Game/FirstPersonBP/Blueprints/FirstPersonCharacter.HealthValue` (+ _healthvalue (`self.AddHealth`)) _characterreference)
  (set `/Game/FirstPersonBP/Blueprints/FirstPersonCharacter.EnergyValue` (+ (`self.AddEnergy`) _healthvalue) _characterreference)
  (set `/Game/FirstPersonBP/Blueprints/FirstPersonCharacter.MoodValue` (+ (`self.AddMood`) (`/Game/FirstPersonBP/Blueprints/FirstPersonCharacter.MoodValue` _characterreference)) _characterreference)
  (`self.K2_DestroyActor`))

(fn `UserConstructionScript`)